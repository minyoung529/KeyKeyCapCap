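; BP_Generator is an enemy spawner for battle that keeps creating BPBoss enemies at a set interval.
; BeginPlay calls EnemyLoop, which starts a looping timer on GenerateEnemy using GenerateTime.
; Each tick of that timer picks a random actor from MousePos, spawns a boss at a fixed offset from it, then passes that actor as its target and initializes its HP widget.
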(event EventBeginPlay
  (CallFunction|EnemyLoop))

(event Collision|EventActorBeginOverlap
  (params (OtherActor :type Actor%20Object%20Reference)))

(event EventTick
  (params (DeltaSeconds :type Float%20%28single-precision%29)))

(fn ConstructionScript)

(fn GenerateEnemy
  (bind _output_get (LocalVariables|SetRandomTargetPos (.OutItem (Utilities|Array|Random (Variables|Generate|GetMousePos)))))
  (bind _returnvalue (Game|SpawnActorfromClass "/Game/Battle/BP/BPBoss.BPBoss_C" (Math|Conversions|ToTransform(Vector) (+ (Transformation|GetActorLocation _output_get) (+ (* (Math|Vector|VectorUp) 2.0) (* (Class|KismetMathLibrary|VectorRight) -1.2e+02)))) "Undefined" 0 0))
  (Class|Enemy|InitTarget _returnvalue (LocalVariables|GetRandomTargetPos))
  (Default|InitHpWidget _returnvalue))

(fn EnemyLoop
  (Utilities|Time|SetTimerbyFunctionName 0 "GenerateEnemy" (Variables|Generate|GetGenerateTime) true))